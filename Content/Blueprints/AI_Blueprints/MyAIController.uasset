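; AI controller for RobotMinion pawns that sends them to a commanded location.
; Every tick it casts the controlled pawn to RobotMinion and checks its AI command enum.
; While that command is active, it prints the move status as debug output and issues a MoveToLocation to the minion's location variable whenever movement is idle.
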(event `self.ReceiveTick`
  (params (DeltaSeconds :type "Float (single-precision)"))
  (bind _returnvalue (`self.GetMoveStatus`))
  (bind _asrobot_minion (cast `/Game/Blueprints/RobotMinion` (`self.K2_GetPawn`)))
  (if (`|EnumEquality` (`/Game/Blueprints/RobotMinion.AIcommand` _asrobot_minion) "NewEnumerator1")
    (`KismetSystemLibrary.PrintString` (`|GetEnumeratorNameAsString` _returnvalue))
    (if (`|EnumEquality` _returnvalue "Idle")
      (`self.MoveToLocation` self (`/Game/Blueprints/RobotMinion.LocationVar` _asrobot_minion) -1.0 true true false true null true))))

(fn `UserConstructionScript`)
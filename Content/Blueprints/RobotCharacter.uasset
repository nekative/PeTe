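; Robot AI character that moves with steering behaviors relative to player character index 1 and can hold branching conversations.
; Each tick, CurrentAction selects a steering component (seek, flee, face, align, arrive, velocity matching, wander) or the Discuss state.
; Discuss checks for a partner, sets up the dialog tree and binds to its HUD's player-choice event.
; Choices update mood and phrase; when dialog ends, mood switches the robot to Wander, Arrive or Flee.
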(event `self.ReceiveTick`
  (params (DeltaSeconds :type "Float (single-precision)"))
  (switch `/Game/Blueprints/AI_Blueprints/RobotActions` (`self.CurrentAction`)
    (:`NewEnumerator1`
      (`/Game/Blueprints/AI_Blueprints/SteeringBehaviourComponents/sbSeek.calculateNewPosition` (`self.sbSeek`) (`self.CharacterMovement`) (`Character.CharacterMovement` (`GameplayStatics.GetPlayerCharacter` 1))))
    (:`NewEnumerator2`
      (`/Game/Blueprints/AI_Blueprints/SteeringBehaviourComponents/sbFlee.calculateNewPosition` (`self.sbFlee`) (`self.CharacterMovement`) (`Character.CharacterMovement` (`GameplayStatics.GetPlayerCharacter` 1))))
    (:`NewEnumerator3`
      (`/Game/Blueprints/AI_Blueprints/SteeringBehaviourComponents/sbFace.calculateNewPosition` (`self.sbFace`) (`self.CharacterMovement`) (`Character.CharacterMovement` (`GameplayStatics.GetPlayerCharacter` 1))))
    (:`NewEnumerator4`
      (`/Game/Blueprints/AI_Blueprints/SteeringBehaviourComponents/sbAlign.calculateNewPosition` (`self.sbAlign`) (`self.CharacterMovement`) (`Character.CharacterMovement` (`GameplayStatics.GetPlayerCharacter` 1))))
    (:`NewEnumerator5`
      (`/Game/Blueprints/AI_Blueprints/SteeringBehaviourComponents/sbArrive.calculateNewPosition` (`self.sbArrive`) (`self.CharacterMovement`) (`Character.CharacterMovement` (`GameplayStatics.GetPlayerCharacter` 1))))
    (:`NewEnumerator6`
      (`/Game/Blueprints/AI_Blueprints/SteeringBehaviourComponents/sbMatchingVelocity.calculateNewPosition` (`self.sbMatchingVelocity`) (`self.CharacterMovement`) (`Character.CharacterMovement` (`GameplayStatics.GetPlayerCharacter` 1))))
    (:`NewEnumerator7`
      (`/Game/Blueprints/AI_Blueprints/SteeringBehaviourComponents/sbWander.Calculate New Position` (`self.sbWander`) (`self.CharacterMovement`)))
    (:`NewEnumerator11`
      (bind _inrange (`/Game/Blueprints/AI_Blueprints/SteeringBehaviourComponents/DialogTree.CheckPartner` (`self.DialogTree`)))
      (if _inrange
        ;[1 1 1] Check if discussion has started already or not
        (if (== (`self.CurrentAIPhrase`) 0)
          ;[1 1 1] Create dialog tree
          (`/Game/Blueprints/AI_Blueprints/SteeringBehaviourComponents/DialogTree.SetUpDialogTree` (`self.DialogTree`))
          ;[1 1 1] Set up current AI phrase from dialog tree
          (set `self.CurrentAIPhrase` (`/Game/Blueprints/AI_Blueprints/SteeringBehaviourComponents/DialogTree.CurrentAIPhraseID` (`self.DialogTree`)))
          ;[1 1 1] Bind event to handle AI's responses (GUI)
          (add `/Game/Blueprints/AI_Blueprints/DTHUD.PlayerSpoke_ED` (`/Game/Blueprints/AI_Blueprints/SteeringBehaviourComponents/DialogTree.DialogTreeHUD` (`self.DialogTree`)) (delegate `CustomEvent_0`)))))))

(event `CustomEvent_0`
  (params (PlayerChoice :type Integer))
  (bind _dialogtree (`self.DialogTree`))
  (bind _dialogtree_2 (`self.DialogTree`))
  ;[1 1 1] After every response of the player + update robot mood for each answer
  (bind _robotmood (`/Game/Blueprints/AI_Blueprints/SteeringBehaviourComponents/DialogTree.UpdateMood` _dialogtree PlayerChoice))
  (`KismetSystemLibrary.PrintString` (`|GetEnumeratorNameAsString` _robotmood))
  (bind _conversationendresult (`/Game/Blueprints/AI_Blueprints/SteeringBehaviourComponents/DialogTree.UpdateDialogTree` _dialogtree PlayerChoice))
  ;[1 1 1] Check if value is negative, if so, disable conversation
  (if (> _conversationendresult 0)
    (set `self.CurrentAIPhrase` (`/Game/Blueprints/AI_Blueprints/SteeringBehaviourComponents/DialogTree.CurrentAIPhraseID` _dialogtree_2))
    (else
      (`/Game/Blueprints/AI_Blueprints/SteeringBehaviourComponents/DialogTree.DisableDialogTree` _dialogtree_2)
      (if (`|EnumEquality` _robotmood "NewEnumerator0")
        (set `self.CurrentAction` "NewEnumerator7")
        (elif (`|EnumEquality` _robotmood "NewEnumerator1")
          (set `self.CurrentAction` "NewEnumerator5")
          (elif (`|EnumEquality` _robotmood "NewEnumerator2")
            (set `self.CurrentAction` "NewEnumerator2")))))))

(fn `UserConstructionScript`)
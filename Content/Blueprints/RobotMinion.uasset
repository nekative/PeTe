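; RobotMinion is an AI minion Blueprint with a set of steering behavior components, though none of them are currently wired to run.
; It starts with its static mesh hidden and LocationVar taken from LocationTarget.
; While HitLoc is true, Tick copies player 1's location into LocationVar and shows the mesh.
; The AIcommand switch has no connected cases, leaving the CurrentAction steering switch and a separate path-follow call unreachable.
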(event `self.ReceiveBeginPlay`
  (set `self.LocationVar` (`self.K2_GetActorLocation` (`self.LocationTarget`)))
  (`SceneComponent.SetVisibility` (`self.StaticMesh`) false false))

(event `self.ReceiveTick`
  (params (DeltaSeconds :type "Float (single-precision)"))
  (if (`self.HitLoc`)
    (set `self.LocationVar` (`CharacterMovementComponent.GetLastUpdateLocation` (`Character.CharacterMovement` (`GameplayStatics.GetPlayerCharacter` 1))))
    (`SceneComponent.SetVisibility` (`self.StaticMesh`) true false))
  (switch `/Game/Blueprints/AI_Blueprints/AIactions` (`self.AIcommand`)))

(fn `UserConstructionScript`)
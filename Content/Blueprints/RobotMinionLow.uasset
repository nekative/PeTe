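; Robot minion character that moves through steering behavior components, either flocking or following the RobotBoss.
; BeginPlay seeds a random planar flocking velocity and turns the actor to face it.
; Each Tick, the Flocking flag selects flocking or leader following, passing CharacterMovement to the chosen component's CalculateNewPosition.
; A CurrentAction switch over other steering behaviors such as seek, flee, wander and path following is left unconnected and never runs.
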(event `self.ReceiveBeginPlay`
  ;[1 1 1] for random movement
  (bind _output_get (set `self.VelocityForFlocking` (`KismetMathLibrary.MakeVector` (`KismetMathLibrary.RandomFloatInRange` 0.4 0.5) (`KismetMathLibrary.RandomFloatInRange` 0.4 0.5))))
  (`self.K2_SetActorRotation` (`KismetMathLibrary.Conv_VectorToRotator` _output_get)))

(event `self.ReceiveTick`
  (params (DeltaSeconds :type "Float (single-precision)"))
  (if (`self.Flocking`)
    (`/Game/Blueprints/AI_Blueprints/SteeringBehaviourComponents/sbFlocking.Calculate New Position` (`self.sbFlocking`) (`self.CharacterMovement`))
    (else
      (`/Game/Blueprints/AI_Blueprints/SteeringBehaviourComponents/sbFollowLeader.calculateNewPosition` (`self.sbFollowLeader`) (`self.CharacterMovement`) (`Character.CharacterMovement` (`self.RobotBoss`))))))

(fn `UserConstructionScript`)